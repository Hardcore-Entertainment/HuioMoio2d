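; Base weapon actor that fires bullets when its owning character shoots.
; On BeginPlay it casts its Instigator to BG_character and binds SpawningProjectile to that character's firing event.
; Each firing event spawns a TestBullet at the weapon's location, using its rotation with a -90 degree yaw offset.
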(event `self.ReceiveBeginPlay`
  (bind _asbg_character (cast `/Game/Blueprints/BG_character` (`self.Instigator`)))
  (add `/Game/Blueprints/BG_character.Firing` _asbg_character (delegate `SpawningProjectile`)))

(event `SpawningProjectile`
  (`|SpawnActorFromClass` "/Game/Blueprints/TestBullet.TestBullet_C" (`KismetMathLibrary.MakeTransform` (.location (`self.GetTransform`)) (`KismetMathLibrary.MakeRotator` (.roll (`self.K2_GetActorRotation`)) (.pitch (`self.K2_GetActorRotation`)) (+ (.yaw (`self.K2_GetActorRotation`)) -90.0))) "Undefined" "OverrideRootScale" null null))

(fn `UserConstructionScript`)