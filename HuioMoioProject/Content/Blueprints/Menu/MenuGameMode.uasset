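; MenuGameMode is the menu game mode that tracks player controllers joining the multiplayer Lobby level.
; On BeginPlay in Lobby it clears its controller list and re-adds the first MenuPlayerController found if that has authority.
; On PostLogin in Lobby it appends the new controller, copies the list to MenuGameState and passes it to that controller's NewPlayerLobbyAdd.
; A loop printing player names is left unconnected.
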(event `self.ReceiveBeginPlay`
  (bind _returnvalue (`GameplayStatics.GetCurrentLevelName` true))
  (switch `string` _returnvalue
    (:`Lobby`
      (`KismetArrayLibrary.Array_Clear` (`self.RefPlayersControllers`))
      (bind _outactors (`GameplayStatics.GetAllActorsOfClass` "/Game/Blueprints/Menu/MenuPlayerController.MenuPlayerController_C"))
      (bind _output (`|GetArrayItem` _outactors))
      (if (`self.HasAuthority` _output)
        (`KismetArrayLibrary.Array_Add` (`self.RefPlayersControllers`) _output)))))

(event `self.ReceiveTick`
  (params (DeltaSeconds :type "Float (single-precision)")))

(event `self.K2_PostLogin`
  (params (NewPlayer :type "PlayerController Object Reference"))
  (bind _asmenu_player_controller (cast `/Game/Blueprints/Menu/MenuPlayerController` NewPlayer :!pure true))
  (bind _refplayerscontrollers (`self.RefPlayersControllers`))
  (bind _returnvalue (`GameplayStatics.GetCurrentLevelName` true))
  (switch `string` _returnvalue
    (:`Lobby`
      (bind _asmenu_game_state (cast `/Game/Blueprints/Menu/MenuGameState` (`GameplayStatics.GetGameState`)))
      (`KismetArrayLibrary.Array_Add` _refplayerscontrollers _asmenu_player_controller)
      (set `/Game/Blueprints/Menu/MenuGameState.PlayerControllers` (`self.RefPlayersControllers`) _asmenu_game_state)
      (`/Game/Blueprints/Menu/MenuPlayerController.NewPlayerLobbyAdd` _asmenu_player_controller _refplayerscontrollers))))

(fn `UserConstructionScript`)