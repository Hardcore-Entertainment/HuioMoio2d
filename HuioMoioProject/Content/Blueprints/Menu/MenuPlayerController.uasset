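; Player controller for the menu and lobby that shows the matching widget by level name and runs online session create, find and join.
; Creating opens Lobby as a listen server, finding feeds results to the MenuButtons session list, and creating or joining removes the current widget.
; In Lobby, BeginPlay and NewPlayerLobbyAdd only print the controllers held by MenuGameState; the chat widget's player refresh is unwired.
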(event `JoinSess`
  (params (SessToJoin :type "BlueprintSessionResult Structure"))
  (`JoinSessionCallbackProxy.JoinSession` self SessToJoin
    (:`OnSuccess`
      (`KismetSystemLibrary.PrintString` "Joined")
      (`Widget.RemoveFromParent` (`self.RefCurrentWidget`) :!label _label))
    (:`OnFailure`
      (`KismetSystemLibrary.PrintString` "Failed"))))

(event `CreateSess`
  (`CreateSessionCallbackProxy.CreateSession` self 10
    (:`OnSuccess`
      (`KismetSystemLibrary.PrintString` "Created")
      (`GameplayStatics.OpenLevel` "Lobby" true "listen")
      (goto _label))
    (:`OnFailure`
      (`KismetSystemLibrary.PrintString` "Failed"))))

(event `FindSess`
  (bind _refmenubuttons (`self.RefMenuButtons`))
  (bind _results (`FindSessionsCallbackProxy.FindSessions` self 10)
    (:`OnSuccess`
      (`KismetSystemLibrary.PrintString` "Found")
      (set `/Game/Widgets/Menu/MenuButtons.RefSessions` _results _refmenubuttons)
      (`/Game/Widgets/Menu/MenuButtons.InitSessionsList` _refmenubuttons))
    (:`OnFailure`
      (`KismetSystemLibrary.PrintString` "Failed"))))

(event `self.ReceiveBeginPlay`
  (bind _returnvalue (`GameplayStatics.GetCurrentLevelName` true))
  (switch `string` _returnvalue
    (:`Menu`
      (bind _returnvalue_2 (`|CreateWidget` "/Game/Widgets/Menu/MenuButtons.MenuButtons_C"))
      (`UserWidget.AddToViewport` _returnvalue_2 0)
      (bind _output_get (set `self.RefMenuButtons` _returnvalue_2))
      (set `self.RefCurrentWidget` _output_get))
    (:`Lobby`
      (bind _returnvalue_3 (`|CreateWidget` "/Game/Widgets/Menu/LobbyChat.LobbyChat_C"))
      (`UserWidget.AddToViewport` _returnvalue_3 0)
      (bind _output_get_2 (set `self.RefLobbyChat` _returnvalue_3))
      (set `self.RefCurrentWidget` _output_get_2)
      (bind _asmenu_game_state (cast `/Game/Blueprints/Menu/MenuGameState` (`GameplayStatics.GetGameState`) :!label _label_2))
      (for _array_element (`/Game/Blueprints/Menu/MenuGameState.PlayerControllers` _asmenu_game_state)
        (`KismetSystemLibrary.PrintString` (`KismetSystemLibrary.GetDisplayName` _array_element))))))

(event `NewPlayerLobbyAdd`
  (params (PlayersControllers :type "Array of /Game/Blueprints/Menu/MenuPlayerController Object Reference"))
  (goto _label_2))

(event `self.ReceiveTick`
  (params (DeltaSeconds :type "Float (single-precision)")))

(fn `UserConstructionScript`)